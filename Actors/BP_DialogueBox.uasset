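; Tutorial trigger box that shows timed French hints on the tank's controls, such as movement, cannon aiming, firing and zoom.
; ShowDialogue creates the WPB_Text widget, displays the welcome message and hides it after a delay.
; When BP_Tank_Player overlaps the box, ChangeText picks the hint matching Number, which shows briefly on that widget.
; HasActivated is set only after that delay, then blocks further triggers.
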(event `self.Show_Dialogue`
  (bind _returnvalue (`|CreateWidget` "/Game/01-Blueprints/UI/WPB_Text.WPB_Text_C"))
  (bind _output_get (set `self.Widget_text` _returnvalue))
  (set `TextBlock.Text` "Bienvenue dans la ville détruite. Déplacez votre Tank avec ZQSD et bougez votre souris pour déplacer la tourelle." (`/Game/01-Blueprints/UI/WPB_Text.TextBlock_0` _output_get))
  (`UserWidget.AddToViewport` _output_get 0)
  (`KismetSystemLibrary.Delay` 3.0)
  (`Widget.SetVisibility` (`self.Widget_text`) "Hidden"))

(event `self.ChangeText`
  (params (number_of_dialogue :type Integer))
  (bind _textblock_0 (`/Game/01-Blueprints/UI/WPB_Text.TextBlock_0` (`self.Widget_text`)))
  (switch `int` number_of_dialogue
    (:`0`
      (set `TextBlock.Text` "Vous pouvez monter/descendre votre canon en appuyant sur E/A. Tirez en appuyant sur le clic droit." _textblock_0))
    (:`1`
      (set `TextBlock.Text` "Le clic gauche vous permettera de viser avec l'angle de vue du canon. Visez cette tourelle ennemie et détruisez la." _textblock_0))
    (:`2`
      (set `TextBlock.Text` "Lorsque vous êtes en vue canon, utilisez la molette pour zoomer/dézoomer." _textblock_0))))

(event `self.BoxComp.OnComponentBeginOverlap`
  (params (OverlappedComponent :type "PrimitiveComponent Object Reference") (OtherActor :type "Actor Object Reference") (OtherComp :type "PrimitiveComponent Object Reference") (OtherBodyIndex :type Integer) (bFromSweep :type Boolean) (SweepResult :type "HitResult Structure (by ref)"))
  (cast `/Game/01-Blueprints/Pawns/BP_Tank_Player` OtherActor)
  (if (not (`self.Has_activated`))
    (`Widget.SetVisibility` (`self.Widget_text`) "Hidden")
    (`self.ChangeText` (`self.number`))
    (`Widget.SetVisibility` (`self.Widget_text`) "Visible")
    (`KismetSystemLibrary.Delay` 3.0)
    (`Widget.SetVisibility` (`self.Widget_text`) "Hidden")
    (`self.Set_HasActivated` true)))

(fn `UserConstructionScript`)