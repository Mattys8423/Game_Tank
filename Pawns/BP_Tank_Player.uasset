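; Player tank pawn Blueprint that shows and hides the aiming and reload UI.
; ActivateAim and ShowReload each create a fresh WBP_Aim or WBP_Reload widget, store it and add it to the viewport.
; DeactivateAim and RemoveReload take the stored widget off screen through the GameViewportSubsystem.
; The graph holds only this UI handling, with no triggers for these events and an empty construction script.
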(event `self.ActivateAim`
  (bind _returnvalue (`|CreateWidget` "/Game/01-Blueprints/UI/WBP_Aim.WBP_Aim_C"))
  (bind _output_get (set `self.Widget_Aim` _returnvalue))
  (`UserWidget.AddToViewport` _output_get 0))

(event `self.DeactivateAim`
  (`GameViewportSubsystem.RemoveWidget` (subsystem `GameViewportSubsystem`) (`self.Widget_Aim`)))

(event `self.ShowReload`
  (bind _returnvalue (`|CreateWidget` "/Game/01-Blueprints/UI/WBP_Reload.WBP_Reload_C"))
  (bind _output_get (set `self.Widget_Reload` _returnvalue))
  (`UserWidget.AddToViewport` _output_get 0))

(event `self.RemoveReload`
  (`GameViewportSubsystem.RemoveWidget` (subsystem `GameViewportSubsystem`) (`self.Widget_Reload`)))

(fn `UserConstructionScript`)